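; Player shooter character Blueprint that adds an intro sound on top of its parent class's behavior.
; On BeginPlay it runs the parent logic, then plays the Intro sound at the character's location in every level except MainMenu, checked by level name.
; Overlap and Tick events are disabled placeholders, and the construction script only calls the parent.
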(event EventBeginPlay
  (|CallParentFunction)
  (bind _returnvalue (Game|GetCurrentLevelName true))
  (if (Utilities|Enum|NotEqual(Enum) _returnvalue "MainMenu")
    (Audio|PlaySoundatLocation "/Game/AssetPacks/GameDevTV/VoiceOvers/Intro.Intro" (Transformation|GetActorLocation) "0, 0, 0" 1.0 1.0 0.0 0 0 0)))

(event Collision|EventActorBeginOverlap
  (params (OtherActor :type Actor%20Object%20Reference))
  (|CallParentFunction OtherActor) ; This node is disabled and will not be called.\nDrag off pins to build functionality.
)

(event EventTick
  (params (DeltaSeconds :type Float%20%28single-precision%29))
  (|CallParentFunction DeltaSeconds) ; This node is disabled and will not be called.\nDrag off pins to build functionality.
)

(fn ConstructionScript
  (|CallParentFunction))